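; BP_Cauldron is a cooking cauldron that collects ingredients and spawns the matching recipe result.
; StartCooking stores each ingredient's ID; from the third onward, up to a fourth, it sorts and concatenates the IDs into a Recipes map key.
; A match spawns the mapped class beside the cauldron and clears the key string.
; The ingredient list is never cleared, nor is the key after a failed lookup.
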(event `/Game/Blueprints/BPI_Cook.StartCooking`
  (params (Object :type "/Game/Objects/InteractableObjects/BP_Ingredient Object Reference"))
  (bind _igredientlist (`self.IgredientList`))
  (bind _igredientlist_2 (`self.IgredientList`))
  (bind _ingredients (`self.Ingredients`))
  (bind _returnvalue (`KismetArrayLibrary.Array_Length` _igredientlist))
  (bind (_value _returnvalue_2) (`BlueprintMapLibrary.Map_Find` (`self.Recipes`) _ingredients))
  ; check amount of ingredients added already
  (bind _output_get (set `self.Igredient` Object))
  (`KismetSystemLibrary.PrintString` "Started cooking")
  (if (< _returnvalue 2)
    (`KismetSystemLibrary.PrintString` "<2")
    (bind _returnvalue_3 (`KismetStringLibrary.Conv_NameToString` (`/Game/Objects/InteractableObjects/BP_Ingredient.GetIngredientID` _output_get)))
    (`KismetArrayLibrary.Array_Add` _igredientlist _returnvalue_3)
    (elif (<= _returnvalue 3)
      (`KismetSystemLibrary.PrintString` "<=3")
      (`KismetArrayLibrary.Array_Add` _igredientlist_2 _returnvalue_3)
      ; Changing array to one string to search map
      (`KismetArrayLibrary.SortStringArray` _igredientlist_2)
      (for _array_element _igredientlist_2
        (set `self.Ingredients` (`KismetStringLibrary.Concat_StrStr` (`self.Ingredients`) _array_element)))
      (`KismetSystemLibrary.DelayUntilNextTick`)
      (`KismetSystemLibrary.PrintString` _ingredients)
      (if _returnvalue_2
        (`KismetSystemLibrary.PrintString` "recipie found")
        (`|SpawnActorFromClass` _value (`KismetMathLibrary.Conv_VectorToTransform` (+ (`SceneComponent.K2_GetComponentLocation` (`self.Cauldron`)) (* (`KismetMathLibrary.Vector_Forward`) 50.0))) "Undefined" "MultiplyWithRoot" null null)
        (`KismetSystemLibrary.PrintString` "Spawned recipe")
        (set `self.Ingredients` "")
        (else
          (`KismetSystemLibrary.PrintString` "recipe not found"))))))

(fn `UserConstructionScript`)