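; BP_SpawnGarlic is an interactable object that dispenses garlic ingredients.
; On StartInteract it waits a zero-length Delay, then spawns a BP_Ingredient_Garlic actor at a fixed world-forward offset from its Sphere component and prints a debug message.
; The event has no limit or cooldown check, and the construction script only calls its parent.
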(event `self.StartInteract`
  ; Spawn new resource
  (`KismetSystemLibrary.Delay` 0.0)
  (`|SpawnActorFromClass` "/Game/Objects/InteractableObjects/BP_Ingredient_Garlic.BP_Ingredient_Garlic_C" (`KismetMathLibrary.Conv_VectorToTransform` (+ (`SceneComponent.K2_GetComponentLocation` (`self.Sphere`)) (* (`KismetMathLibrary.Vector_Forward`) 50.0))) "Undefined" "MultiplyWithRoot" null "4" null)
  (`KismetSystemLibrary.PrintString` "spawned"))

(fn `UserConstructionScript`
  (`parent.UserConstructionScript`))